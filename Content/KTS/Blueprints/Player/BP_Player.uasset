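; BP_Player is the player character, handling movement, camera look and interaction through Enhanced Input.
; On BeginPlay, once the input subsystem is valid, it adds IMC_Player and spawns a BP_ZipTail attached to the mesh's TailSocket.
; Look input yaws the CameraArm in world space, and move input follows the camera's right and forward vectors.
; Starting the interact action fires CallOnInteract.
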(event `self.ReceiveBeginPlay`
  (bind _mesh (`self.Mesh`))
  (bind _returnvalue (pcsubsystem `EnhancedInputLocalPlayerSubsystem` (cast `PlayerController` (`self.GetController`) :!pure true)))
  (`/Engine/EditorBlueprintResources/StandardMacros.IsValid` _returnvalue
    (:`Is Valid`
      (`EnhancedInputSubsystemInterface.AddMappingContext` _returnvalue "/Game/KTS/Blueprints/Player/Controls/IMC_Player.IMC_Player" 0 (struct))
      (bind _returnvalue_2 (`|SpawnActorFromClass` "/Game/KTS/Blueprints/Characters/Zip/BP_ZipTail.BP_ZipTail_C" (`SceneComponent.GetSocketTransform` _mesh "TailSocket" "RTS_World") "Undefined" "MultiplyWithRoot" null null))
      (`self.K2_AttachToComponent` _returnvalue_2 _mesh "TailSocket" "SnapToTarget" "SnapToTarget" "SnapToTarget" true))))

(event `EnhancedInput|/Game/KTS/Blueprints/Player/Controls/Actions/IA_Look`
  (params (ActionValue :type "Vector2D Structure") (ElapsedSeconds :type "Float (double-precision)") (TriggeredSeconds :type "Float (double-precision)") (InputAction :type "InputAction Object Reference" :default "/Game/KTS/Blueprints/Player/Controls/Actions/IA_Look.IA_Look"))
  (:`Triggered`
    (`SceneComponent.K2_AddWorldRotation` (`self.CameraArm`) (`KismetMathLibrary.MakeRotator` 0.0 0.0 ActionValue_X) false false)))

(event `EnhancedInput|/Game/KTS/Blueprints/Player/Controls/Actions/IA_Move`
  (params (ActionValue :type "Vector2D Structure") (ElapsedSeconds :type "Float (double-precision)") (TriggeredSeconds :type "Float (double-precision)") (InputAction :type "InputAction Object Reference" :default "/Game/KTS/Blueprints/Player/Controls/Actions/IA_Move.IA_Move"))
  (bind _camera (`self.Camera`))
  (:`Triggered`
    (`self.AddMovementInput` (`KismetMathLibrary.GetRightVector` (`SceneComponent.K2_GetComponentRotation` _camera)) ActionValue_X)
    (`self.AddMovementInput` (`KismetMathLibrary.GetForwardVector` (`SceneComponent.K2_GetComponentRotation` _camera)) ActionValue_Y)))

(event `EnhancedInput|/Game/KTS/Blueprints/Player/Controls/Actions/IA_Interact`
  (params (ActionValue :type Boolean) (ElapsedSeconds :type "Float (double-precision)") (TriggeredSeconds :type "Float (double-precision)") (InputAction :type "InputAction Object Reference" :default "/Game/KTS/Blueprints/Player/Controls/Actions/IA_Interact.IA_Interact"))
  (:`Started`
    (`self.OnInteract`)))

(fn `UserConstructionScript`)