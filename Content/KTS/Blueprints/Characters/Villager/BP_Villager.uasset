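; BP_Villager is a villager character with a Mass agent component and placeholder reactions to player interaction and fear.
; On BeginPlay it gives its mesh a dynamic material with a random fully saturated hue.
; Any sphere overlap binds Interact to BP_Player's interact event, with no unbinding on exit; Interact only prints a greeting.
; Scared prints the same greeting and deactivates the MassAgent; physics and UI widget logic are unconnected.
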(event `self.ReceiveBeginPlay`
  (bind _returnvalue (`PrimitiveComponent.CreateDynamicMaterialInstance` (`self.Mesh`) 0 "/Game/KTS/Blueprints/Characters/Villager/M_Villager.M_Villager" "None"))
  (bind _output_get (set `self.Material` _returnvalue))
  (`MaterialInstanceDynamic.SetVectorParameterValue` _output_get "Color" (`KismetMathLibrary.HSVToRGB` (`KismetMathLibrary.RandomFloatInRange` 0.0 360.0) 1.0 1.0)))

(event `self.Sphere.OnComponentBeginOverlap`
  (params (OverlappedComponent :type "PrimitiveComponent Object Reference") (OtherActor :type "Actor Object Reference") (OtherComp :type "PrimitiveComponent Object Reference") (OtherBodyIndex :type Integer) (bFromSweep :type Boolean) (SweepResult :type "HitResult Structure (by ref)"))
  (add `/Game/KTS/Blueprints/Player/BP_Player.OnInteract` (cast `/Game/KTS/Blueprints/Player/BP_Player` (`GameplayStatics.GetPlayerCharacter` 0) :!pure true) (delegate `/Game/KTS/Blueprints/Characters/BP_Interact.Interact`)))

(event `/Game/KTS/Blueprints/Characters/BP_Interact.Interact`
  (`KismetSystemLibrary.PrintString` "Hello"))

(event `self.Sphere.OnComponentEndOverlap`
  (params (OverlappedComponent :type "PrimitiveComponent Object Reference") (OtherActor :type "Actor Object Reference") (OtherComp :type "PrimitiveComponent Object Reference") (OtherBodyIndex :type Integer)))

(event `Scared`
  (`KismetSystemLibrary.PrintString` "Hello")
  (`ActorComponent.Deactivate` (`self.MassAgent`)))

(fn `UserConstructionScript`)