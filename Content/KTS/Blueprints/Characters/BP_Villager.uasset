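; BP_Villager is a villager character that offers player interaction and dialogue through the Mountea Dialogue system.
; Entering its Sphere binds the player's OnInteract to an Interact event, which currently only prints "Hello".
; Leaving the Sphere unbinds all OnInteract listeners, then initializes the participant, requests the dialogue widget and starts dialogue between player and villager.
; A separate WB_UIWidget creation chain is unconnected and never runs.
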(event `self.Sphere.OnComponentBeginOverlap`
  (params (OverlappedComponent :type "PrimitiveComponent Object Reference") (OtherActor :type "Actor Object Reference") (OtherComp :type "PrimitiveComponent Object Reference") (OtherBodyIndex :type Integer) (bFromSweep :type Boolean) (SweepResult :type "HitResult Structure (by ref)"))
  (add `/Game/KTS/Blueprints/Player/BP_Player.OnInteract` (cast `/Game/KTS/Blueprints/Player/BP_Player` (`GameplayStatics.GetPlayerCharacter` 0) :!pure true) (delegate `/Game/KTS/Blueprints/Characters/BP_Interact.Interact`)))

(event `/Game/KTS/Blueprints/Characters/BP_Interact.Interact`
  (`KismetSystemLibrary.PrintString` "Hello"))

(event `self.Sphere.OnComponentEndOverlap`
  (params (OverlappedComponent :type "PrimitiveComponent Object Reference") (OtherActor :type "Actor Object Reference") (OtherComp :type "PrimitiveComponent Object Reference") (OtherBodyIndex :type Integer))
  (bind _mounteadialoguemanager (`self.MounteaDialogueManager`))
  (bind _asbp_player (cast `/Game/KTS/Blueprints/Player/BP_Player` (`GameplayStatics.GetPlayerCharacter` 0) :!pure true))
  (clear `/Game/KTS/Blueprints/Player/BP_Player.OnInteract` _asbp_player)
  (`MounteaDialogueParticipantStatics.InitializeParticipant` (`self.MounteaDialogueParticipant`) _mounteadialoguemanager)
  (`MounteaDialogueHUDStatics.RequestShowWidget` _mounteadialoguemanager (`self.Fade Progress Duration`))
  (`MounteaDialogueManagerStatics.RequestStartDialogue` _mounteadialoguemanager _asbp_player (make `DialogueParticipants` _asbp_player (`|MakeArray` self))))

(fn `UserConstructionScript`)